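; Game mode for a Smashers match that sets up game-only input, music and the in-game UI, and runs the round timer.
; On BeginPlay it branches on the selected game mode: Story saves level data to the game instance, Two Players creates a second local player, and any other non-Online mode spawns an AI controller.
; Tick counts down the timer while active and opens the time-finished menu level when it expires.
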(event `self.ReceiveBeginPlay`
  (bind _returnvalue (`GameplayStatics.GetPlayerController` 0))
  (set `PlayerController.bShowMouseCursor` false _returnvalue)
  (`WidgetBlueprintLibrary.SetInputMode_GameOnly` _returnvalue)
  (`GameplayStatics.PlaySound2D` "/Game/Assets/Music/Smashers/SC/SC_GameMusic.SC_GameMusic" 1.0 1.0 0.0 null null)
  (bind _returnvalue_2 (`|CreateWidget` "/Game/Blueprints/Widget/InGameUI/BP_InGameUI.BP_InGameUI_C"))
  (`UserWidget.AddToViewport` _returnvalue_2 0)
  (bind _returnvalue_3 (`GameModeSelectionSystem.GetGm` (subsystem `GameModeSelectionSystem`)))
  (if (== _returnvalue_3 "Story")
    (bind _returnvalue_4 (`self.GetLevelData`))
    (message `SaveGameInterface.SaveLevelData` (`GameplayStatics.GetGameInstance`) _returnvalue_4)
    (elif (== _returnvalue_3 "Two Players")
      (`GameplayStatics.CreatePlayer` 1)
      (elif (not (== _returnvalue_3 "Online"))
        (`|SpawnActorFromClass` "/Game/Blueprints/AI/BP_SmashersAIController.BP_SmashersAIController_C" (`KismetMathLibrary.MakeTransform` (0.0 0.0 0.0)) "Undefined" "MultiplyWithRoot" null null)))))

(event `self.ReceiveTick`
  (params (DeltaSeconds :type "Float (single-precision)"))
  (if (`self.TimerActive`)
    (bind _output_get (set `self.RoundTimer` (- (`self.RoundTimer`) DeltaSeconds)))
    (if (<= _output_get 0.0)
      (`GameplayStatics.OpenLevel` "TimeFinishedMenu"))))

(fn `UserConstructionScript`)