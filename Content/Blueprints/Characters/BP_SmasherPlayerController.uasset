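; BP_SmasherPlayerController is a player controller that provides the pause menu toggle.
; Shortly after BeginPlay it creates a BP_PauseScreen widget, stores it, adds it to the viewport and hides it.
; Releasing P or Gamepad Special Right toggles game pause, widget visibility and input mode, giving the screen keyboard focus when shown.
; The toggle finds the widget through GetAllWidgetsOfClass instead of the stored PauseWidget reference.
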(event `self.ReceiveBeginPlay`
  (if true
    (`KismetSystemLibrary.Delay` 0.2)
    (bind _returnvalue (`|CreateWidget` "/Game/Blueprints/Widget/PauseScreen/BP_PauseScreen.BP_PauseScreen_C" (`GameplayStatics.GetPlayerController` 0)))
    (bind _output_get (set `self.PauseWidget` _returnvalue))
    (`UserWidget.AddToViewport` _output_get 0)
    (`UserWidget.AddToViewport` _returnvalue 0)
    (`Widget.SetVisibility` _output_get "Hidden")
    (`Widget.SetVisibility` _returnvalue "Hidden")))

(event `Key|Gamepad_Special_Right` :paused true
  (params (Key :type "Key Structure"))
  (bind _returnvalue (`GameplayStatics.GetPlayerController` 0))
  (:`Released`
    (if (`GameplayStatics.IsGamePaused`) :!label _label
      (bind _foundwidgets (`WidgetBlueprintLibrary.GetAllWidgetsOfClass` "/Game/Blueprints/Widget/PauseScreen/BP_PauseScreen.BP_PauseScreen_C"))
      (`Widget.SetVisibility` _foundwidgets "Hidden")
      (`WidgetBlueprintLibrary.SetInputMode_GameOnly` _returnvalue)
      (`GameplayStatics.SetGamePaused` false)
      (else
        (bind _foundwidgets_2 (`WidgetBlueprintLibrary.GetAllWidgetsOfClass` "/Game/Blueprints/Widget/PauseScreen/BP_PauseScreen.BP_PauseScreen_C"))
        (`Widget.SetVisibility` _foundwidgets_2 "Visible")
        (`Widget.SetKeyboardFocus` _foundwidgets_2)
        (`WidgetBlueprintLibrary.SetInputMode_GameAndUIEx` _returnvalue null)
        (`GameplayStatics.SetGamePaused` true)))))

(event `Key|P`
  (params (Key :type "Key Structure"))
  (:`Released`
    (goto _label)))

(fn `UserConstructionScript`)