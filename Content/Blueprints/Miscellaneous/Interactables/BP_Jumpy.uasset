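; BP_Jumpy is an interactable pickup that temporarily boosts the jump speed of a SmashersPlayerCharacter.
; Interact calls UpdateMovementParams with a fixed amount added to the current jump speed and zero for walk and run speeds, then waits InteractDuration.
; EndInteract makes the same call with that amount subtracted from the then-current jump speed, then destroys the actor.
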(event `self.Interact`
  (params (SmashersPlayerCharacter :type "SmashersPlayerCharacter Object Reference"))
  (`SmashersPlayerCharacter.UpdateMovementParams` SmashersPlayerCharacter 0.0 0.0 (+ (`SmashersPlayerCharacter.JumpSpeed` SmashersPlayerCharacter) 250.0))
  (`KismetSystemLibrary.Delay` (`self.InteractDuration`))
  (`self.EndInteract` SmashersPlayerCharacter))

(event `self.EndInteract`
  (params (SmashersPlayerCharacter :type "SmashersPlayerCharacter Object Reference"))
  (`SmashersPlayerCharacter.UpdateMovementParams` SmashersPlayerCharacter 0.0 0.0 (- (`SmashersPlayerCharacter.JumpSpeed` SmashersPlayerCharacter) 250.0))
  (`self.K2_DestroyActor`))

(fn `UserConstructionScript`)