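; BP_AttackIncrement is an interactable pickup that temporarily doubles the interacting Smashers player's attack damage.
; Interact doubles heavy and light damage on the player's AttackComponent, waits InteractDuration, then calls EndInteract.
; EndInteract halves both values to undo the boost and destroys the actor, which therefore stays alive for the whole buff.
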(event `self.Interact`
  (params (SmashersPlayerCharacter :type "SmashersPlayerCharacter Object Reference"))
  (bind _attackcomponent (`SmashersPlayerCharacter.AttackComponent` SmashersPlayerCharacter))
  (set `AttackComponent.HeavyAttackDamage` (* (`AttackComponent.HeavyAttackDamage` _attackcomponent) 2.0) _attackcomponent)
  (set `AttackComponent.LightAttackDamage` (* (`AttackComponent.LightAttackDamage` _attackcomponent) 2.0) _attackcomponent)
  (`KismetSystemLibrary.Delay` (`self.InteractDuration`))
  (`self.EndInteract` SmashersPlayerCharacter))

(event `self.EndInteract`
  (params (SmashersPlayerCharacter :type "SmashersPlayerCharacter Object Reference"))
  (bind _attackcomponent (`SmashersPlayerCharacter.AttackComponent` SmashersPlayerCharacter))
  (set `AttackComponent.HeavyAttackDamage` (* (`AttackComponent.HeavyAttackDamage` _attackcomponent) 0.5) _attackcomponent)
  (set `AttackComponent.LightAttackDamage` (* (`AttackComponent.LightAttackDamage` _attackcomponent) 0.5) _attackcomponent)
  (`self.K2_DestroyActor`))

(fn `UserConstructionScript`)